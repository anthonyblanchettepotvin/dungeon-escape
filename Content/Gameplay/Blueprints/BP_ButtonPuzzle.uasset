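; BP_ButtonPuzzle is a puzzle controller that unlocks or relocks a reward actor based on whether all its conditions are met.
; Every Tick it evaluates each Conditions entry through the PuzzleCondition interface, failing on the first false result; non-implementers only print a warning.
; On a change of state it calls UnlockReward or LockReward on Reward through the PuzzleReward interface, checking the current lock state first.
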(event EventBeginPlay)

(event Collision|EventActorBeginOverlap
  (params (OtherActor :type Actor%20Object%20Reference)))

(event EventTick
  (params (DeltaSeconds :type Float%20%28single-precision%29))
  (bind _returnvalue (CallFunction|ConditionsMet))
  (if _returnvalue
    (if (not (Variables|Puzzle|GetIsConditionsMet))
      (Class|Puzzle|OnConditionsMet)
      (Variables|Puzzle|SetIsConditionsMet true))
    (elif (Variables|Puzzle|GetIsConditionsMet)
      (Class|Puzzle|OnConditionsUnmet)
      (Variables|Puzzle|SetIsConditionsMet false))))

(event EventOnConditionsMet
  (if (Variables|Puzzle|GetIsActorPuzzleReward)
    (bind _aspuzzle_reward (Utilities|Casting|CastToPuzzleReward (Variables|Puzzle|GetReward))
      (:then
        (bind _returnvalue (Class|PuzzleReward|IsRewardUnlocked _aspuzzle_reward))
        (if (not _returnvalue)
          (Class|PuzzleReward|UnlockReward _aspuzzle_reward)))
      (:CastFailed
        (Variables|Puzzle|SetIsActorPuzzleReward false)
        (Development|PrintString "Object doesn't implement IPuzzleReward.")))))

(event EventOnConditionsUnmet
  (if (Variables|Puzzle|GetIsActorPuzzleReward)
    (bind _aspuzzle_reward (Utilities|Casting|CastToPuzzleReward (Variables|Puzzle|GetReward))
      (:then
        (bind _returnvalue (Class|PuzzleReward|IsRewardUnlocked _aspuzzle_reward))
        (if _returnvalue
          (Class|PuzzleReward|LockReward _aspuzzle_reward)))
      (:CastFailed
        (Variables|Puzzle|SetIsActorPuzzleReward false)
        (Development|PrintString "Object doesn't implement IPuzzleReward.")))))

(fn ConstructionScript)

(fn ConditionsMet
  (for _array_element (Variables|Puzzle|GetConditions)
    (bind _aspuzzle_condition (Utilities|Casting|CastToPuzzleCondition _array_element)
      (:then
        (bind _returnvalue (Class|PuzzleCondition|Evaluate _aspuzzle_condition))
        (if (not _returnvalue)
          (return false)))
      (:CastFailed
        (Development|PrintString "Object doesn't implement IPuzzleCondition."))))
  (return true))