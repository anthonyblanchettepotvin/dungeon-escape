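; Pressure plate Blueprint that reports whether enough physical weight rests on its Trigger.
; Evaluate loops over actors overlapping the Trigger and adds the mass of each one's first found primitive component, if it simulates physics.
; It returns true when the total reaches TargetMass.
; The event graph and construction script are empty, so nothing in this Blueprint calls Evaluate.
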(event EventBeginPlay)

(event Collision|EventActorBeginOverlap
  (params (OtherActor :type Actor%20Object%20Reference)))

(event EventTick
  (params (DeltaSeconds :type Float%20%28single-precision%29)))

(fn ConstructionScript)

(fn Evaluate
  (for _array_element (Collision|GetOverlappingActors (Variables|Default|GetTrigger) 0 :!class /Script/Engine.Actor)
    (if (Physics|IsSimulatingPhysics (Actor|GetComponentbyClass _array_element "/Script/Engine.PrimitiveComponent") "None")
      (LocalVariables|SetTotalMass (+ (LocalVariables|GetTotalMass) (Physics|GetMass (Actor|GetComponentbyClass _array_element "/Script/Engine.PrimitiveComponent"))))))
  (return (>= (LocalVariables|GetTotalMass) (Variables|Default|GetTargetMass))))