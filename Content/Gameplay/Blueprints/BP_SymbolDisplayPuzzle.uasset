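; BP_SymbolDisplayPuzzle is a puzzle controller that locks or unlocks a reward based on a set of conditions.
; Every tick it evaluates each entry in Conditions as a PuzzleCondition, requiring all to pass.
; An AlreadyMet flag limits action to state changes, calling UnlockReward or LockReward on the PuzzleReward and firing OnConditionsMet or OnConditionsUnmet.
; Both events currently only print debug messages.
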(event EventBeginPlay)

(event Collision|EventActorBeginOverlap
  (params (OtherActor :type Actor%20Object%20Reference)))

(event EventTick
  (params (DeltaSeconds :type Float%20%28single-precision%29))
  (bind _returnvalue (CallFunction|ConditionsMet))
  (if _returnvalue
    (if (not (Variables|Puzzle|GetAlreadyMet))
      (bind _aspuzzle_reward (Utilities|Casting|CastToPuzzleReward (Variables|Puzzle|GetReward)))
      (Class|PuzzleReward|UnlockReward _aspuzzle_reward)
      (Variables|Puzzle|SetAlreadyMet true)
      (Class|Puzzle|OnConditionsMet))
    (elif (Variables|Puzzle|GetAlreadyMet)
      (bind _aspuzzle_reward_2 (Utilities|Casting|CastToPuzzleReward (Variables|Puzzle|GetReward)))
      (Class|PuzzleReward|LockReward _aspuzzle_reward_2)
      (Variables|Puzzle|SetAlreadyMet false)
      (Class|Puzzle|OnConditionsUnmet))))

(event EventOnConditionsUnmet
  (Development|PrintString "Symbol Display Puzzle: Conditions Unmet."))

(event EventOnConditionsMet
  (Development|PrintString "Symbol Display Puzzle: Conditions Met."))

(fn ConstructionScript)

(fn ConditionsMet
  (for _array_element (Variables|Puzzle|GetConditions)
    (bind _aspuzzle_condition (Utilities|Casting|CastToPuzzleCondition _array_element))
    (bind _returnvalue (Class|PuzzleCondition|Evaluate _aspuzzle_condition))
    (if (not _returnvalue)
      (return false)))
  (return true))