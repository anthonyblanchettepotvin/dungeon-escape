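; BP_Button is an interactable toggle button that moves between a raised and a pressed position and tracks its pressed state.
; On BeginPlay it stores the Button component's world location as the rest position.
; Interact alternates between Press, which snaps the component to that position minus the TargetPosition offset, and Unpress, which restores it, then always returns false.
; Evaluate exposes the IsPressed state to callers.
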(event EventBeginPlay
  (Variables|Button|SetInitialPosition (Transformation|GetWorldLocation (Variables|Default|GetButton))))

(event Collision|EventActorBeginOverlap
  (params (OtherActor :type Actor%20Object%20Reference)))

(event EventTick
  (params (DeltaSeconds :type Float%20%28single-precision%29)))

(fn ConstructionScript)

(fn Unpress
  (Transformation|SetWorldLocation (Variables|Default|GetButton) (Variables|Button|GetInitialPosition) false false)
  (Variables|Button|SetIsPressed false))

(fn Press
  (Transformation|SetWorldLocation (Variables|Default|GetButton) (- (Variables|Button|GetInitialPosition) (Variables|Button|GetTargetPosition)) false false)
  (Variables|Button|SetIsPressed true))

(fn Evaluate
  (return (Variables|Button|GetIsPressed)))

(fn Interact
  (if (Variables|Button|GetIsPressed)
    (Button|Unpress)
    (else
      (Button|Press)))
  (return false))