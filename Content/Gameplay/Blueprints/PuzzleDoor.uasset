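; Puzzle door that unlocks and opens while all of its puzzle conditions are met, and locks and closes when one fails.
; Every tick it evaluates the Conditions array through PuzzleConditionInterface, skipping elements that do not implement it.
; An IsConditionsMet flag limits the open and close events to state changes.
; The Interact override calls the parent's interaction only while the door is unlocked.
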(event EventBeginPlay
  (|CallParentFunction) ; This node is disabled and will not be called.\nDrag off pins to build functionality.
)

(event Collision|EventActorBeginOverlap
  (params (OtherActor :type Actor%20Object%20Reference))
  (|CallParentFunction OtherActor) ; This node is disabled and will not be called.\nDrag off pins to build functionality.
)

(event EventTick
  (params (DeltaSeconds :type Float%20%28single-precision%29))
  (|CallParentFunction DeltaSeconds)
  (CallFunction|ConditionsMet))

(event EventOnConditionsMet
  (Variables|Default|SetbIsUnlocked true)
  (Class|DoorComponent|OpenDoor (Variables|Default|GetDoor)))

(event EventOnConditionsUnmet
  (Variables|Default|SetbIsUnlocked false)
  (Class|DoorComponent|CloseDoor (Variables|Default|GetDoor)))

(fn ConstructionScript
  (|CallParentFunction))

(fn Interact
  (if (Variables|Default|GetbIsUnlocked)
    (|CallParentFunction)
    (return false)))

(fn ConditionsMet
  (for _array_element (Variables|Default|GetConditions)
    (if (Utilities|DoesObjectImplementInterface _array_element "/Script/TempleEscape.PuzzleConditionInterface")
      (bind _aspuzzle_condition_interface (Utilities|Casting|CastToPuzzleConditionInterface _array_element))
      (bind _returnvalue (Class|PuzzleConditionInterface|Evaluate _aspuzzle_condition_interface))
      (if (not _returnvalue)
        (if (Variables|Default|GetbIsConditionsMet)
          (Variables|Default|SetbIsConditionsMet false)
          (Class|PuzzleInterface|OnConditionsUnmet))
        (return false))))
  (if (not (Variables|Default|GetbIsConditionsMet))
    (Variables|Default|SetbIsConditionsMet true)
    (Class|PuzzleInterface|OnConditionsMet))
  (return true))