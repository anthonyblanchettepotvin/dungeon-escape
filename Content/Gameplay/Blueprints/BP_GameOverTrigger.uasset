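; BP_GameOverTrigger is an overlap trigger that ends the Temple Escape game when the player reaches it carrying the golden gargoyle.
; On overlap by the first player character, it compares that character's GrabberComponent GrabbedActor against the GoldenGargoyleActor reference.
; A match calls GameOver on BP_TempleEscapeGameState; otherwise the game state shows a timed reminder message not to forget the gargoyle.
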(event EventBeginPlay)

(event Collision|EventActorBeginOverlap
  (params (OtherActor :type Actor%20Object%20Reference))
  (bind _returnvalue (Game|GetPlayerCharacter 0))
  (if (== OtherActor _returnvalue)
    (bind _asbp_temple_escape_game_state (Utilities|Casting|CastToBP_TempleEscapeGameState (Game|GetGameState)))
    (if (== (Variables|/Script/TempleEscape.GrabberComponent|GetGrabbedActor (Actor|GetComponentbyClass _returnvalue "/Script/TempleEscape.GrabberComponent")) (Variables|Default|GetGoldenGargoyleActor))
      (Default|GameOver _asbp_temple_escape_game_state)
      (else
        (Default|ShowMessage _asbp_temple_escape_game_state 0 "I must not forget the golden gargoyle." 5.0)))))

(event EventTick
  (params (DeltaSeconds :type Float%20%28single-precision%29)))

(fn ConstructionScript)