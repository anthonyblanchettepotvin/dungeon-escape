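; Interactable puzzle torch that toggles between lit and extinguished, flipping its neighbour torches too, Lights Out style.
; Interact triggers the toggle, which propagates only one level to valid Neighbours.
; Light and Extinguish switch the fire particles and point light, then report IsLit through the PuzzleCondition component, flagging it as changing state meanwhile.
; BeginPlay applies the initial state without propagation and binds to BP_TorchesTrigger's extinguish event, which puts the torch out.
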(event Custom|Event%20OnExtinguishTorches
  (CallFunction|Extinguish false))

(event EventBeginPlay
  (|CallParentFunction)
  (if (Variables|Default|GetIsLit)
    (CallFunction|Light false)
    (else
      (CallFunction|Extinguish false)))
  (bind _returnvalue (Actor|GetActorOfClass "/Game/Gameplay/Blueprints/BP_TorchesTrigger.BP_TorchesTrigger_C"))
  (EventDispatchers|BindEventtoExtinguishTorches _returnvalue (delegate Custom|Event%20OnExtinguishTorches)))

(event Collision|EventActorBeginOverlap
  (params (OtherActor :type Actor%20Object%20Reference))
  (|CallParentFunction OtherActor) ; This node is disabled and will not be called.\nDrag off pins to build functionality.
)

(event EventTick
  (params (DeltaSeconds :type Float%20%28single-precision%29))
  (|CallParentFunction DeltaSeconds) ; This node is disabled and will not be called.\nDrag off pins to build functionality.
)

(fn ConstructionScript
  (|CallParentFunction))

(fn Light
  (params (InfluenceNeighbours :type Boolean))
  (bind _torch_pointlight (Variables|Default|GetTorch_PointLight))
  (Class|PuzzleConditionComponent|SetIsChangingState (Variables|Default|GetPuzzleCondition) true)
  (Components|Activation|Activate (Variables|Default|GetP_Torch_Fire) false)
  (Components|Activation|Activate _torch_pointlight false)
  (Rendering|Components|Light|SetIntensity _torch_pointlight 5e+03)
  (if InfluenceNeighbours
    (CallFunction|InfluenceNeighbours))
  (Class|PuzzleConditionComponent|SetIsChangingState (Variables|Default|GetPuzzleCondition) false)
  (bind _output_get (Variables|Default|SetIsLit true))
  (Class|PuzzleConditionComponent|NotifyStateChanged (Variables|Default|GetPuzzleCondition) _output_get))

(fn Extinguish
  (params (InfluenceNeighbours :type Boolean))
  (bind _torch_pointlight (Variables|Default|GetTorch_PointLight))
  (Class|PuzzleConditionComponent|SetIsChangingState (Variables|Default|GetPuzzleCondition) true)
  (Components|Activation|Deactivate (Variables|Default|GetP_Torch_Fire))
  (Components|Activation|Deactivate _torch_pointlight)
  (Rendering|Components|Light|SetIntensity _torch_pointlight 0.0)
  (if InfluenceNeighbours
    (CallFunction|InfluenceNeighbours))
  (Class|PuzzleConditionComponent|SetIsChangingState (Variables|Default|GetPuzzleCondition) false)
  (bind _output_get (Variables|Default|SetIsLit false))
  (Class|PuzzleConditionComponent|NotifyStateChanged (Variables|Default|GetPuzzleCondition) _output_get))

(fn LightExtinguish
  (params (InfluenceNeighbours :type Boolean))
  (if (Variables|Default|GetIsLit)
    (CallFunction|Extinguish InfluenceNeighbours)
    (else
      (CallFunction|Light InfluenceNeighbours))))

(fn InfluenceNeighbours
  (for _array_element (Variables|Default|GetNeighbours)
    (if (Utilities|IsValid _array_element)
      (CallFunction|LightExtinguish _array_element false))))

(fn Interact
  (CallFunction|LightExtinguish true)
  (return true))